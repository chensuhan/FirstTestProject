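; Story manager that prepares narrative data and the player's save when play begins.
; BeginPlay flattens DT_Story and each row's nested PlotData table into StoryList, one entry per row holding its stage and plot list.
; It then loads the BP_StorySaveGame slot, or creates and saves one if none exists.
; StoryInit seeds a new save with initial attribute values from DT_Attribute and every DT_Item entry set to false.
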(event `self.ReceiveBeginPlay`
  (`|ExecutionSequence`
    (:`then_0`
      (bind _outrownames (`DataTableFunctionLibrary.GetDataTableRowNames` "/Game/Story/Blueprints/Data/Story/DT_Story.DT_Story"))
      (for _array_element _outrownames
        (bind _returnvalue (`|GetDataTableRow` "/Game/Story/Blueprints/Data/Story/DT_Story.DT_Story" _array_element)
          (:`then`
            (bind (_stage _plotdata) (break `/Game/Story/Blueprints/Data/Struct/ST_Story` _returnvalue))
            (set `self.StoryStage` _stage)
            (bind _outrownames_2 (`DataTableFunctionLibrary.GetDataTableRowNames` _plotdata))
            (for _array_element_2 _outrownames_2
              (bind _returnvalue_2 (`|GetDataTableRow` _plotdata _array_element_2)
                (:`then`
                  (`KismetArrayLibrary.Array_AddUnique` (`self.PlotList`) _returnvalue_2))))
            (`KismetArrayLibrary.Array_AddUnique` (`self.StoryList`) (make `/Game/Story/Blueprints/Core/Struct/ST_C_Story` (`self.StoryStage`) (`self.PlotList`)))
            (set `self.StoryStage` -1)
            (`KismetArrayLibrary.Array_Clear` (`self.PlotList`))))))
    (:`then_1`
      (bind _returnvalue_3 (`GameplayStatics.DoesSaveGameExist` "SaveGame"))
      (if _returnvalue_3
        (bind _returnvalue_4 (`GameplayStatics.LoadGameFromSlot` "SaveGame"))
        (bind _asbp_story_save_game (cast `/Game/Story/Blueprints/GameFramework/BP_StorySaveGame` _returnvalue_4))
        (set `self.SaveGame` _asbp_story_save_game)
        (else
          (`self.Story Init`)
          (`GameplayStatics.SaveGameToSlot` (`self.SaveGame`) "SaveGame"))))))

(fn `Story Init`
  (bind _returnvalue (`GameplayStatics.CreateSaveGameObject` "/Game/Story/Blueprints/GameFramework/BP_StorySaveGame.BP_StorySaveGame_C"))
  (set `self.SaveGame` _returnvalue)
  (`|ExecutionSequence`
    (:`then_0`
      (bind _outrownames (`DataTableFunctionLibrary.GetDataTableRowNames` "/Game/Story/Blueprints/Data/DT_Attribute.DT_Attribute"))
      (for _array_element _outrownames
        (bind _returnvalue_2 (`|GetDataTableRow` "/Game/Story/Blueprints/Data/DT_Attribute.DT_Attribute" _array_element)
          (:`then`
            (bind (_id _describe _initial) (break `/Game/Story/Blueprints/Data/Struct/ST_Attribute` _returnvalue_2))
            (`BlueprintMapLibrary.Map_Add` (`/Game/Story/Blueprints/GameFramework/BP_StorySaveGame.Attribute` (`self.SaveGame`)) _id _initial)))))
    (:`then_1`
      (bind _outrownames_2 (`DataTableFunctionLibrary.GetDataTableRowNames` "/Game/Story/Blueprints/Data/DT_Item.DT_Item"))
      (for _array_element_2 _outrownames_2
        (bind _returnvalue_3 (`|GetDataTableRow` "/Game/Story/Blueprints/Data/DT_Item.DT_Item" _array_element_2)
          (:`then`
            (`BlueprintMapLibrary.Map_Add` (`/Game/Story/Blueprints/GameFramework/BP_StorySaveGame.Item` (`self.SaveGame`)) (`.ID_6_8E5EF45F4D4C75460290D2A45B1AC0CD` (break `/Game/Story/Blueprints/Data/Struct/ST_Item` _returnvalue_3)))))))))

(fn `UserConstructionScript`)